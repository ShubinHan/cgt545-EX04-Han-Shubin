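; Spawner pad that places a collectible energy orb at its own location when the collection game starts.
; On BeginPlay it binds to the StartGame event of GM_CollectionGame, then spawns BP_EnergyOrb_Collectible either immediately or through a one-shot timer when delayed spawning is enabled.
; The pad mesh swaps a material slot to metal while waiting on a delay and to glow once the orb spawns.
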(event Custom|StartGame
  (if (Variables|Default|GetDelaySpawn?)
    (CallFunction|DelayedSpawn)
    (else
      (CallFunction|Spawn))))

(event EventBeginPlay
  (bind _asgm_collection_game (Utilities|Casting|CastToGM_CollectionGame (Game|GetGameMode)))
  (bind _output_get (Variables|Default|SetGame%20Mode _asgm_collection_game))
  (EventDispatchers|BindEventtoStartGame _output_get (EventDispatchers|CreateEvent :!event Custom|StartGame)))

(event EventSpawn
  (Game|SpawnActorfromClass "/Game/GameplayMechanics/Blueprints/BP_EnergyOrb_Collectible.BP_EnergyOrb_Collectible_C" (Math|Transform|MakeTransform (Transformation|GetActorLocation) "0, 0, 0" "1.000000,1.000000,1.000000") "Undefined" self 0)
  (Rendering|Material|SetMaterial (Variables|Default|GetPadMesh) 1 "/Game/StackOBot/Environment/Materials/MI_Glow.MI_Glow"))

(event EventDelayedSpawn
  (Rendering|Material|SetMaterial (Variables|Default|GetPadMesh) 1 "/Game/StackOBot/Environment/Materials/MI_Metal.MI_Metal")
  (Utilities|Time|SetTimerbyEvent (delegate EventSpawn) (Variables|Default|GetSpawnDelay)))

(fn ConstructionScript)