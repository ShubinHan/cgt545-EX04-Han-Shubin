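; GM_CollectionGame runs the rules of a timed collection game, won by reaching a target score before time runs out.
; The game stays paused from BeginPlay until StartGame_Event unpauses it, starts a one-shot timer and calls the StartGame dispatcher.
; CheckScore sets Win on an exact TargetScore match and triggers the end, while timer expiry triggers it as a loss.
; EndGame_Event pauses the timer and game, then calls the EndGame dispatcher.
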(event Custom|TimerEnd
  (Variables|Default|SetWin false)
  (Development|PrintString "Lose-End Timer")
  (CallFunction|EndGameEvent))

(event Custom|StartGame_Event
  (Game|SetGamePaused false)
  (bind _returnvalue (Utilities|Time|SetTimerbyEvent (delegate Custom|TimerEnd) (Variables|Default|GetGameTime)))
  (Variables|Default|SetGame%20Timer _returnvalue)
  (Default|CallStartGame))

(event Custom|EndGame_Event
  (Utilities|Time|PauseTimerbyHandle (Variables|Default|GetGame%20Timer))
  (Game|SetGamePaused true)
  (Default|CallEndGame))

(event EventBeginPlay
  (Game|SetGamePaused true))

(event EventTick
  (params (DeltaSeconds :type Float%20%28single-precision%29)))

(fn ConstructionScript)

(fn CheckScore
  (params (Score :type Integer))
  (bind _output_get (Variables|Default|SetWin (== Score (Variables|Default|GetTargetScore))))
  (if _output_get
    (CallFunction|EndGameEvent)))