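; BP_EnergyOrb_Collectible is a pickup orb for the collection game mode that destroys itself when the game ends.
; A spawn timeline raises and scales it on BeginPlay.
; Overlapping an actor with BPC_Collection that can pick up triggers the pickup once, plays a sound and signals the orb's owner via DelayedSpawnMessage.
; A second timeline then arcs the orb toward the moving collector while scaling it, then destroys it.
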(event Custom|EndGame
  (Actor|DestroyActor))

(event EventBeginPlay
  (|CallParentFunction)
  (bind _asgm_collection_game (Utilities|Casting|CastToGM_CollectionGame (Game|GetGameMode)))
  (bind _output_get (Variables|Default|SetGame%20Mode _asgm_collection_game))
  (EventDispatchers|BindEventtoEndGame _output_get (EventDispatchers|CreateEvent :!event Custom|EndGame))
  (Variables|Default|SetPickupLocation (Transformation|GetActorLocation))
  (bind (_direction _hightalpha _scale) (Timeline|TL_Spawn Play)
    (:Update
      (Transformation|SetActorLocation (Math|Vector|Lerp(Vector) (Variables|Default|GetPickupLocation) (+ (Variables|Default|GetPickupLocation) "0,0,80.000000") _hightalpha) false false)
      (Transformation|SetActorScale3D (Math|Conversions|ToVector(Float) _scale)))
    (:Finished
      (Variables|Default|SetPickupLocation (Transformation|GetActorLocation)))))

(event Collision|EventActorBeginOverlap
  (params (OtherActor :type Actor%20Object%20Reference))
  (bind _returnvalue (Actor|GetComponentbyClass OtherActor "/Game/GameplayMechanics/Blueprints/BPC_Collection.BPC_Collection_C"))
  (Utilities|IsValid _returnvalue
    (:Is%20Valid
      (Variables|Default|SetCollector _returnvalue)
      (Utilities|FlowControl|DoOnce false :!label _label
        (:Completed
          (if (Variables|/Game/GameplayMechanics/Blueprints/BPC_Collection.BPC_Collection_C|GetCanPickUp (Variables|Default|GetCollector))
            (Default|PickUp (Variables|Default|GetCollector))
            (Audio|Components|Audio|Play (Variables|Default|GetSFX_CollectCoin) 0.0)
            (Class|BPIPickup|DelayedSpawn(Message) (Components|GetOwner))
            (bind (_direction _distancealpha _hightalpha _scale) (Timeline|TL_PickUp PlayFromStart)
              (:Update
                (Utilities|IsValid (Components|GetOwner (Variables|Default|GetCollector))
                  (:Is%20Valid
                    (Transformation|SetActorTransform (Math|Transform|MakeTransform (+ (Math|Vector|Lerp(Vector) (Variables|Default|GetPickupLocation) (Transformation|GetActorLocation (Components|GetOwner (Variables|Default|GetCollector))) _distancealpha) (Math|Vector|MakeVector 0.0 0.0 (* _hightalpha 3e+02))) (Transformation|GetActorRotation) (Math|Conversions|ToVector(Float) _scale))))))
              (:Finished
                (Actor|DestroyActor)))
            (else
              (goto _label Reset))))))))

(event EventTick
  (params (DeltaSeconds :type Float%20%28single-precision%29))
  (|CallParentFunction DeltaSeconds) ; This node is disabled and will not be called.\nDrag off pins to build functionality.
)

(fn ConstructionScript
  (|CallParentFunction))