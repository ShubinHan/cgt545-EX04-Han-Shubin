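; BP_DeliveryPoint is a drop-off point that takes carried items from any actor with a BPC_Collection component entering its sphere.
; A timeline arcs a temporary orb mesh from the collector to the point, then calls Deliver on that component.
; A cooldown timer re-arms delivery and repeats it while the collector still overlaps.
; On exit, clearing the collector reference is deferred tick by tick until any running delivery finishes.
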(event OnComponentBeginOverlap(Sphere)
  (params (OverlappedComponent :type Primitive%20Component%20Object%20Reference) (OtherActor :type Actor%20Object%20Reference) (OtherComp :type Primitive%20Component%20Object%20Reference) (OtherBodyIndex :type Integer) (bFromSweep :type Boolean) (SweepResult :type Hit%20Result%20Structure%20%28by%20ref%29))
  (bind _returnvalue (Actor|GetComponentbyClass OtherActor "/Game/GameplayMechanics/Blueprints/BPC_Collection.BPC_Collection_C"))
  (Utilities|IsValid _returnvalue
    (:Is%20Valid
      (bind _output_get (Variables|Default|SetCollector _returnvalue))
      (if (and (> (Variables|/Game/GameplayMechanics/Blueprints/BPC_Collection.BPC_Collection_C|GetCarrying _output_get) 0) (Variables|Default|GetAllowCore))
        (Variables|Default|SetAllowCore false)
        (bind _returnvalue_2 (AddComponent|AddStaticMeshComponent false (Math|Transform|MakeRelativeTransform (Transformation|GetActorTransform (Components|GetOwner (Variables|Default|GetCollector))) (Transformation|GetActorTransform))))
        (Variables|Default|SetOrb _returnvalue_2)
        (Variables|Default|SetOrb%20Start%20Location (.Location (Math|Transform|BreakTransform (Math|Transform|MakeRelativeTransform (Transformation|GetActorTransform (Components|GetOwner (Variables|Default|GetCollector))) (Transformation|GetActorTransform)))))
        (Variables|Default|SetDeliveryInProgress true)
        (bind (_direction _distancealpha _heightalpha _scale) (Timeline|TL_Delivery PlayFromStart)
          (:Update
            (Transformation|SetRelativeTransform (Variables|Default|GetOrb) (Math|Transform|MakeTransform (+ (Math|Vector|Lerp(Vector) (Variables|Default|GetOrb%20Start%20Location) "0, 0, 0" _distancealpha) (Math|Vector|MakeVector 0.0 0.0 (* _heightalpha 3e+02))) "0, 0, 0" (Math|Conversions|ToVector(Float) _scale)) false false))
          (:Finished
            (Components|DestroyComponent (Variables|Default|GetOrb))
            (Default|Deliver (Variables|Default|GetCollector))
            (Variables|Default|SetDeliveryInProgress false)
            (Utilities|Time|SetTimerbyEvent (delegate Custom|ResetAllowScore) (Variables|Default|GetScoreDelay))))))))

(event OnComponentEndOverlap(Sphere)
  (params (OverlappedComponent :type Primitive%20Component%20Object%20Reference) (OtherActor :type Actor%20Object%20Reference) (OtherComp :type Primitive%20Component%20Object%20Reference) (OtherBodyIndex :type Integer))
  (Utilities|IsValid (Variables|Default|GetCollector)
    (:Is%20Valid
      (if (== (Actor|GetComponentbyClass OtherActor "/Game/GameplayMechanics/Blueprints/BPC_Collection.BPC_Collection_C") (Variables|Default|GetCollector))
        (if (Variables|Default|GetDeliveryInProgress) :!label _label
          (Utilities|FlowControl|DelayUntilNextTick)
          (goto _label)
          (else
            (Variables|Default|SetCollector 0)))))))

(event Custom|ResetAllowScore
  (bind _collector (Variables|Default|GetCollector))
  (Variables|Default|SetAllowCore true)
  (Utilities|IsValid _collector
    (:Is%20Valid
      (if (Collision|IsOverlappingActor (Variables|Default|GetSphere) (Components|GetOwner _collector) :!class /Script/Engine.PrimitiveComponent)
        (CallFunction|StartDelivery)))))

(event Custom|StartDelivery
  (bind _returnvalue (Transformation|GetActorTransform))
  (bind _collector (Variables|Default|GetCollector))
  (bind _returnvalue_2 (Components|GetOwner _collector))
  (bind _returnvalue_3 (Transformation|GetActorTransform _returnvalue_2))
  (bind _returnvalue_4 (Math|Transform|MakeRelativeTransform _returnvalue_3 _returnvalue))
  (if (and (> (Variables|/Game/GameplayMechanics/Blueprints/BPC_Collection.BPC_Collection_C|GetCarrying (stale OnComponentBeginOverlap(Sphere) _output_get)) 0) (Variables|Default|GetAllowCore))
    (Variables|Default|SetAllowCore false)
    (bind _returnvalue_5 (AddComponent|AddStaticMeshComponent false _returnvalue_4))
    (Variables|Default|SetOrb _returnvalue_5)
    (Variables|Default|SetOrb%20Start%20Location (.Location (Math|Transform|BreakTransform _returnvalue_4)))
    (Variables|Default|SetDeliveryInProgress true)
    (bind (_direction _distancealpha _heightalpha _scale) (Timeline|TL_Delivery PlayFromStart)
      (:Update
        (Transformation|SetRelativeTransform (Variables|Default|GetOrb) (Math|Transform|MakeTransform (+ (Math|Vector|Lerp(Vector) (Variables|Default|GetOrb%20Start%20Location) "0, 0, 0" _distancealpha) (Math|Vector|MakeVector 0.0 0.0 (* _heightalpha 3e+02))) "0, 0, 0" (Math|Conversions|ToVector(Float) _scale)) false false))
      (:Finished
        (Components|DestroyComponent (Variables|Default|GetOrb))
        (Default|Deliver (Variables|Default|GetCollector))
        (Variables|Default|SetDeliveryInProgress false)
        (Utilities|Time|SetTimerbyEvent (delegate Custom|ResetAllowScore) (Variables|Default|GetScoreDelay))))))

(event EventBeginPlay)

(event Collision|EventActorBeginOverlap
  (params (OtherActor :type Actor%20Object%20Reference)))

(event EventTick
  (params (DeltaSeconds :type Float%20%28single-precision%29)))

(fn ConstructionScript)