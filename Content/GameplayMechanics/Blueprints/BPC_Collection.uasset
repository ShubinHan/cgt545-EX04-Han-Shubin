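; BPC_Collection is a Blueprint that tracks how many items its owner is carrying against a capacity limit.
; Its PickUp event increments Carrying and prints the new count to screen.
; When the count equals Capacity, it clears CanPickUp and prints a capacity message.
; BeginPlay and Tick are empty, and the graph contains no drop or reset logic.
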(event Custom|PickUp
  (bind _output_get (Variables|Default|SetCarrying (+ (Variables|Default|GetCarrying) 1)))
  (Development|PrintString (Utilities|String|Append "Carrying: " (Utilities|String|ToString(Integer) _output_get)))
  (if (== (Variables|Default|GetCarrying) (Variables|Default|GetCapacity))
    (Variables|Default|SetCanPickUp false)
    (Development|PrintString "Capacity reach")))

(event EventBeginPlay)

(event EventTick
  (params (DeltaSeconds :type Float%20%28single-precision%29)))