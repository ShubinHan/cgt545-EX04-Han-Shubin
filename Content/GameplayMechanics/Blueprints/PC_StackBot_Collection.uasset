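; Player controller for the StackBot collection game that manages start and end screens, pawn spawning and camera pitch limits.
; It binds to GM_CollectionGame's start and end events, spawning and possessing the default pawn on start, then destroying it on end and showing the win-dependent end screen.
; Key input depends on which screen exists: any key starts from the start screen, while Enter restarts and Escape quits from the end screen.
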(event Custom|StartGame
  (bind _outactors (Actor|GetAllActorsOfClass "/Script/Engine.PlayerStart"))
  (bind _returnvalue (Game|SpawnActorfromClass (Variables|/Script/Engine.GameModeBase|GetDefaultPawnClass (Variables|Default|GetGame%20Mode)) (Transformation|GetActorTransform (Utilities|Array|Get(acopy) _outactors)) "Undefined" 0 0))
  (Pawn|Possess _returnvalue)
  (Utilities|IsValid (Variables|Default|GetStart%20Screen)
    (:Is%20Valid
      (Widget|RemovefromParent (Variables|Default|GetStart%20Screen))
      (Variables|Default|SetStart%20Screen 0))))

(event Custom|EndGame
  (Viewport|RemoveAllWidgets)
  (bind _returnvalue (UserInterface|CreateWidget "/Game/GameplayMechanics/HUD/UI_EndScreen.UI_EndScreen_C" self))
  (bind _output_get (Variables|Default|SetEndScreen _returnvalue))
  (UserInterface|Viewport|AddtoViewport _output_get 0)
  (Default|SetEndScreenText (Variables|Default|GetEndScreen) (Variables|/Game/GameplayMechanics/Blueprints/GM_CollectionGame.GM_CollectionGame_C|GetWin (Variables|Default|GetGame%20Mode)))
  (Actor|DestroyActor (Pawn|GetControlledPawn)))

(event EventBeginPlay
  (bind _playercameramanager (Variables|Default|GetPlayerCameraManager))
  (Variables|/Script/Engine.PlayerCameraManager|SetViewPitchMin _playercameramanager -65.0)
  (Variables|/Script/Engine.PlayerCameraManager|SetViewPitchMax _playercameramanager 1e+01)
  (bind _asgm_collection_game (Utilities|Casting|CastToGM_CollectionGame (Game|GetGameMode)))
  (bind _output_get (Variables|Default|SetGame%20Mode _asgm_collection_game))
  (EventDispatchers|BindEventtoStartGame _output_get (EventDispatchers|CreateEvent :!event Custom|StartGame))
  (EventDispatchers|BindEventtoEndGame _output_get (EventDispatchers|CreateEvent :!event Custom|EndGame))
  (bind _returnvalue (UserInterface|CreateWidget "/Game/GameplayMechanics/HUD/UI_StartScreen.UI_StartScreen_C" self))
  (bind _output_get_2 (Variables|Default|SetStart%20Screen _returnvalue))
  (UserInterface|Viewport|AddtoViewport _output_get_2 0))

(event EventTick
  (params (DeltaSeconds :type Float%20%28single-precision%29)))

(event Input|KeyboardEvents|AnyKey
  (params (Key :type Key%20Structure :default "None"))
  (:Pressed
    (Utilities|IsValid (Variables|Default|GetStart%20Screen)
      (:Is%20Valid
        (Default|StartGameEvent (Variables|Default|GetGame%20Mode))))))

(event Input|KeyboardEvents|Enter
  (params (Key :type Key%20Structure :default "None"))
  (:Pressed
    (Utilities|IsValid (Variables|Default|GetEndScreen)
      (:Is%20Valid
        (Widget|RemovefromParent (Variables|Default|GetEndScreen))
        (Variables|Default|SetEndScreen 0)
        (Default|StartGameEvent (Variables|Default|GetGame%20Mode))))))

(event Input|KeyboardEvents|Escape
  (params (Key :type Key%20Structure :default "None"))
  (:Pressed
    (Utilities|IsValid (Variables|Default|GetEndScreen)
      (:Is%20Valid
        (Game|QuitGame self "Quit" false)))))

(fn ConstructionScript)